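; First-person player character with movement, object inspection, footstep and ambient audio, and debug view-mode switching.
; Interact traces for "Interactable" actors, moves a child-actor copy to the camera for inspection, then respawns it and lerps it down to the surface below.
; A looping timer runs the footstep timeline while moving, and FootstepsTrace selects sounds from surface flags.
; Tick plays delayed random eerie noises; number keys switch view modes, shown in a widget.
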(event Custom|Reset%20DoOnce
  (bind _item_actor (Variables|Default|GetItem%20Actor))
  ;[0.15 0.15 0.15 0.5] PickUp/PutDown Object
  (Utilities|FlowControl|DoOnce false) ; enters at Reset
)

(event Custom|Inspect
  (bind _item_actor (Variables|Default|GetItem%20Actor))
  (bind _fps_camera (Variables|Default|GetFPS_Camera))
  (bind _returnvalue (Transformation|GetWorldLocation _fps_camera))
  ;[0.15 0.15 0.15 0.5] PickUp/PutDown Object
  (bind (_outhit _returnvalue_2) (Collision|LineTraceByChannel _returnvalue (+ _returnvalue (* (Math|Vector|GetForwardVector _fps_camera) 2.5e+02)) "TraceTypeQuery1" false 0 "None"))
  (if _returnvalue_2
    (if (Actor|ActorHasTag (.HitActor (Collision|BreakHitResult _outhit)) "Interactable")
      (Utilities|FlowControl|Sequence
        (:then_0
          (Utilities|FlowControl|Delay 0.1)
          (if (not (Variables|Default|GetInspecting?))
            (Variables|Default|SetInspecting? true)
            (Variables|Default|SetStart%20Location (Variables|/Script/Engine.SceneComponent|GetRelativeLocation (Variables|Default|GetItem%20Actor)))
            (Variables|Default|SetEnd%20Location (Variables|/Script/Engine.SceneComponent|GetRelativeLocation (Variables|Default|GetArrow1)))
            (bind _item_track (Timeline|Pick%20Up%20Item Play)
              (:Update
                (Transformation|SetRelativeLocation (Variables|Default|GetItem%20Actor) (Math|Vector|Lerp(Vector) (Variables|Default|GetStart%20Location) (Variables|Default|GetEnd%20Location) _item_track) false false))
              (:Finished
                (if (Variables|Default|GetInspecting?)
                  (bind _asbp_inspectable_parent (Utilities|Casting|CastToBP_InspectableParent (Variables|/Script/Engine.ChildActorComponent|GetChildActor (Variables|Default|GetItem%20Actor))))
                  (Default|StartInspect _asbp_inspectable_parent self)
                  (else
                    (bind _returnvalue_3 (Game|SpawnActorfromClass (Variables|/Script/Engine.ChildActorComponent|GetChildActorClass (Variables|Default|GetItem%20Actor)) (Math|Transform|MakeTransform (Math|Transform|TransformLocation (Transformation|GetWorldTransform (Variables|Default|GetFPS_Camera)) (Variables|/Script/Engine.SceneComponent|GetRelativeLocation (Variables|Default|GetItem%20Actor)))) "Undefined" "MultiplyWithRoot" 0 0))
                    (Variables|Default|SetPlacedItem _returnvalue_3)
                    (ChildActorComponent|SetChildActorClass (Variables|Default|GetItem%20Actor) 0)
                    (CallFunction|ResetDoOnce)
                    (bind _outhit_2 (Collision|LineTraceByChannel (Transformation|GetActorLocation (Variables|Default|GetPlacedItem)) (- (Transformation|GetActorLocation (Variables|Default|GetPlacedItem)) "0.000000,0.000000,1000.000000") "TraceTypeQuery1" false (Utilities|Array|MakeArray (Variables|Default|GetPlacedItem)) "None"))
                    (Variables|Default|SetNewEndLocation (.Location (Collision|BreakHitResult _outhit_2)))
                    (Variables|Default|SetNewStartLocation (Transformation|GetActorLocation (Variables|Default|GetPlacedItem)))
                    (bind _fixlocation_track (Timeline|FixLocation PlayFromStart)
                      (:Update
                        (Transformation|SetActorLocation (Variables|Default|GetPlacedItem) (Math|Vector|Lerp(Vector) (Variables|Default|GetNewStartLocation) (Variables|Default|GetNewEndLocation) _fixlocation_track) false false)))))))
            (else
              (Variables|Default|SetInspecting? false)
              (Timeline|Pick%20Up%20Item Reverse))))
        (:then_1
          (Utilities|FlowControl|DoOnce false
            (:Completed
              (ChildActorComponent|SetChildActorClass _item_actor (Utilities|GetClass (.HitActor (Collision|BreakHitResult _outhit))))
              (Transformation|SetRelativeLocation _item_actor (Math|Transform|InverseTransformLocation (Transformation|GetWorldTransform (Variables|Default|GetFPS_Camera)) (Transformation|GetActorLocation (.HitActor (Collision|BreakHitResult _outhit)))) false false)
              (Actor|DestroyActor (.HitActor (Collision|BreakHitResult _outhit))))))))))

(event Custom|Footsteps%20Timer
  ;[0.15 0.15 0.15 0.5] Play Footsteps in time with walk speed
  (Utilities|Time|SetTimerbyEvent (delegate Custom|CheckForFootstep) 0.01 true))

(event Custom|CheckForFootstep
  (bind _tl_footsteps (Variables|Default|GetTL_Footsteps))
  ;[0.15 0.15 0.15 0.5] Play Footsteps in time with walk speed
  (if (> (Math|Vector|VectorLengthXY (Variables|/Script/Engine.MovementComponent|GetVelocity (Variables|Character|GetCharacterMovement))) 0.0)
    (Components|Timeline|SetPlayRate _tl_footsteps 1.0)
    (Audio|Components|Audio|Play _tl_footsteps)
    (else
      (Audio|Components|Audio|Stop (Variables|Default|GetTL_Footsteps)))))

(event EventBeginPlay
  (bind _views (Variables|Default|GetViews))
  ;[0.15 0.15 0.15 0.5] Start footstep timer
  (Utilities|FlowControl|Sequence
    (:then_0
      (CallFunction|FootstepsTimer))
    (:then_1
      ;[0.15 0.15 0.15 0.5] View types
      (Utilities|Array|Add _views "viewmode lit")
      (Utilities|Array|Add _views "viewmode unlit")
      (Utilities|Array|Add _views "viewmode wireframe")
      (Utilities|Array|Add _views "viewmode lit_wireframe")
      (Utilities|Array|Add _views "viewmode lit_detaillighting")
      (Utilities|Array|Add _views "viewmode lightingonly")
      (Utilities|Array|Add _views "viewmode lightcomplexity")
      (Utilities|Array|Add _views "viewmode shadercomplexity")
      ;[0.15 0.15 0.15 0.5] Set View Mode widget
      (bind _returnvalue (UserInterface|CreateWidget "/Game/Individual_Work/Piper/WB_ViewMode.WB_ViewMode_C"))
      (UserInterface|Viewport|AddtoViewport _returnvalue 0))))

(event EventTick
  (params (DeltaSeconds :type Float%20%28single-precision%29))
  ;[0.15 0.15 0.15 0.5] Play Eerie noises randomly (30-40s)
  (Utilities|FlowControl|Delay (Math|Random|RandomFloatinRange 3e+01 4e+01))
  (bind _randomlocation (Class|NavigationSystemV1|GetRandomLocationinNavigableRadius (Transformation|GetActorLocation) 1e+02 0 0))
  (Audio|PlaySoundatLocation "/Game/Individual_Work/Piper/Sounds/AMB/SC_AMB_Eerie_Noise.SC_AMB_Eerie_Noise" _randomlocation "0, 0, 0" 1.0 1.0 0.0 0 0 0 0))

(event Input|ActionEvents|InputActionInteract
  (params (Key :type Key%20Structure :default "None"))
  (bind _item_actor (Variables|Default|GetItem%20Actor))
  (bind _fps_camera (Variables|Default|GetFPS_Camera))
  (bind _returnvalue (Transformation|GetWorldLocation _fps_camera))
  ;[0.15 0.15 0.15 0.5] PickUp/PutDown Object
  (:Pressed
    (bind (_outhit _returnvalue_2) (Collision|LineTraceByChannel _returnvalue (+ _returnvalue (* (Math|Vector|GetForwardVector _fps_camera) 2.5e+02)) "TraceTypeQuery1" false 0 "None"))
    (if _returnvalue_2
      (if (Actor|ActorHasTag (.HitActor (Collision|BreakHitResult _outhit)) "Interactable")
        (Utilities|FlowControl|Sequence
          (:then_0
            (Utilities|FlowControl|Delay 0.1)
            (if (not (Variables|Default|GetInspecting?))
              (Variables|Default|SetInspecting? true)
              (Variables|Default|SetStart%20Location (Variables|/Script/Engine.SceneComponent|GetRelativeLocation (Variables|Default|GetItem%20Actor)))
              (Variables|Default|SetEnd%20Location (Variables|/Script/Engine.SceneComponent|GetRelativeLocation (Variables|Default|GetArrow1)))
              (bind _item_track (Timeline|Pick%20Up%20Item Play)
                (:Update
                  (Transformation|SetRelativeLocation (Variables|Default|GetItem%20Actor) (Math|Vector|Lerp(Vector) (Variables|Default|GetStart%20Location) (Variables|Default|GetEnd%20Location) _item_track) false false))
                (:Finished
                  (if (Variables|Default|GetInspecting?)
                    (bind _asbp_inspectable_parent (Utilities|Casting|CastToBP_InspectableParent (Variables|/Script/Engine.ChildActorComponent|GetChildActor (Variables|Default|GetItem%20Actor))))
                    (Default|StartInspect _asbp_inspectable_parent self)
                    (else
                      (bind _returnvalue_3 (Game|SpawnActorfromClass (Variables|/Script/Engine.ChildActorComponent|GetChildActorClass (Variables|Default|GetItem%20Actor)) (Math|Transform|MakeTransform (Math|Transform|TransformLocation (Transformation|GetWorldTransform (Variables|Default|GetFPS_Camera)) (Variables|/Script/Engine.SceneComponent|GetRelativeLocation (Variables|Default|GetItem%20Actor)))) "Undefined" "MultiplyWithRoot" 0 0))
                      (Variables|Default|SetPlacedItem _returnvalue_3)
                      (ChildActorComponent|SetChildActorClass (Variables|Default|GetItem%20Actor) 0)
                      (CallFunction|ResetDoOnce)
                      (bind _outhit_2 (Collision|LineTraceByChannel (Transformation|GetActorLocation (Variables|Default|GetPlacedItem)) (- (Transformation|GetActorLocation (Variables|Default|GetPlacedItem)) "0.000000,0.000000,1000.000000") "TraceTypeQuery1" false (Utilities|Array|MakeArray (Variables|Default|GetPlacedItem)) "None"))
                      (Variables|Default|SetNewEndLocation (.Location (Collision|BreakHitResult _outhit_2)))
                      (Variables|Default|SetNewStartLocation (Transformation|GetActorLocation (Variables|Default|GetPlacedItem)))
                      (bind _fixlocation_track (Timeline|FixLocation PlayFromStart)
                        (:Update
                          (Transformation|SetActorLocation (Variables|Default|GetPlacedItem) (Math|Vector|Lerp(Vector) (Variables|Default|GetNewStartLocation) (Variables|Default|GetNewEndLocation) _fixlocation_track) false false)))))))
              (else
                (Variables|Default|SetInspecting? false)
                (Timeline|Pick%20Up%20Item Reverse))))
          (:then_1
            (Utilities|FlowControl|DoOnce false
              (:Completed
                (ChildActorComponent|SetChildActorClass _item_actor (Utilities|GetClass (.HitActor (Collision|BreakHitResult _outhit))))
                (Transformation|SetRelativeLocation _item_actor (Math|Transform|InverseTransformLocation (Transformation|GetWorldTransform (Variables|Default|GetFPS_Camera)) (Transformation|GetActorLocation (.HitActor (Collision|BreakHitResult _outhit)))) false false)
                (Actor|DestroyActor (.HitActor (Collision|BreakHitResult _outhit)))))))))))

(event Input|AxisEvents|InputAxisLookUp
  (params (AxisValue :type Float%20%28single-precision%29))
  ;[0.15 0.15 0.15 0.5] Camera
  (if (not (Variables|Default|GetPlayerPaused))
    (Pawn|Input|AddControllerPitchInput (* AxisValue 0.3))))

(event Input|AxisEvents|InputAxisMoveForward
  (params (AxisValue :type Float%20%28single-precision%29))
  ;[0.15 0.15 0.15 0.5] Movement
  (if (not (Variables|Default|GetPlayerPaused))
    (Pawn|Input|AddMovementInput (Math|Vector|GetForwardVector (Variables|Collision|GetCapsuleComponent)) AxisValue false)))

(event Input|AxisEvents|InputAxisMoveRight
  (params (AxisValue :type Float%20%28single-precision%29))
  ;[0.15 0.15 0.15 0.5] Movement
  (if (not (Variables|Default|GetPlayerPaused))
    (Pawn|Input|AddMovementInput (Math|Vector|GetRightVector (Variables|Collision|GetCapsuleComponent)) AxisValue false)))

(event Input|AxisEvents|InputAxisTurn
  (params (AxisValue :type Float%20%28single-precision%29))
  ;[0.15 0.15 0.15 0.5] Camera
  (if (not (Variables|Default|GetPlayerPaused))
    (Pawn|Input|AddControllerYawInput (* AxisValue 0.3))))

(event Input|KeyboardEvents|1
  (params (Key :type Key%20Structure :default "None"))
  (bind _views (Variables|Default|GetViews))
  (bind _output (Utilities|Array|Get(acopy) _views))
  ;[0.15 0.15 0.15 0.5] Toggle through views
  (:Pressed
    (if (not (Variables|Default|GetPlayerPaused))
      (Development|ExecuteConsoleCommand _output 0)
      (Rendering|Components|TextRender|SetText (Variables|/Game/Individual_Work/Piper/WB_ViewMode.WB_ViewMode_C|GetViewtype (stale EventBeginPlay _returnvalue)) (Utilities|Text|ToText(String) _output)))))

(event Input|KeyboardEvents|2
  (params (Key :type Key%20Structure :default "None"))
  (bind _views (Variables|Default|GetViews))
  (bind _output (Utilities|Array|Get(acopy) _views 1))
  ;[0.15 0.15 0.15 0.5] Toggle through views
  (:Pressed
    (if (not (Variables|Default|GetPlayerPaused))
      (Development|ExecuteConsoleCommand _output 0)
      (Rendering|Components|TextRender|SetText (Variables|/Game/Individual_Work/Piper/WB_ViewMode.WB_ViewMode_C|GetViewtype (stale EventBeginPlay _returnvalue)) (Utilities|Text|ToText(String) _output)))))

(event Input|KeyboardEvents|3
  (params (Key :type Key%20Structure :default "None"))
  (bind _views (Variables|Default|GetViews))
  (bind _output (Utilities|Array|Get(acopy) _views 2))
  ;[0.15 0.15 0.15 0.5] Toggle through views
  (:Pressed
    (if (not (Variables|Default|GetPlayerPaused))
      (Development|ExecuteConsoleCommand _output 0)
      (Rendering|Components|TextRender|SetText (Variables|/Game/Individual_Work/Piper/WB_ViewMode.WB_ViewMode_C|GetViewtype (stale EventBeginPlay _returnvalue)) (Utilities|Text|ToText(String) _output)))))

(event Input|KeyboardEvents|4
  (params (Key :type Key%20Structure :default "None"))
  (bind _views (Variables|Default|GetViews))
  (bind _output (Utilities|Array|Get(acopy) _views 3))
  ;[0.15 0.15 0.15 0.5] Toggle through views
  (:Pressed
    (if (not (Variables|Default|GetPlayerPaused))
      (Development|ExecuteConsoleCommand _output 0)
      (Rendering|Components|TextRender|SetText (Variables|/Game/Individual_Work/Piper/WB_ViewMode.WB_ViewMode_C|GetViewtype (stale EventBeginPlay _returnvalue)) (Utilities|Text|ToText(String) _output)))))

(event Input|KeyboardEvents|5
  (params (Key :type Key%20Structure :default "None"))
  (bind _views (Variables|Default|GetViews))
  (bind _output (Utilities|Array|Get(acopy) _views 4))
  ;[0.15 0.15 0.15 0.5] Toggle through views
  (:Pressed
    (if (not (Variables|Default|GetPlayerPaused))
      (Development|ExecuteConsoleCommand _output 0)
      (Rendering|Components|TextRender|SetText (Variables|/Game/Individual_Work/Piper/WB_ViewMode.WB_ViewMode_C|GetViewtype (stale EventBeginPlay _returnvalue)) (Utilities|Text|ToText(String) _output)))))

(event Input|KeyboardEvents|6
  (params (Key :type Key%20Structure :default "None"))
  (bind _views (Variables|Default|GetViews))
  (bind _output (Utilities|Array|Get(acopy) _views 5))
  ;[0.15 0.15 0.15 0.5] Toggle through views
  (:Pressed
    (if (not (Variables|Default|GetPlayerPaused))
      (Development|ExecuteConsoleCommand _output 0)
      (Rendering|Components|TextRender|SetText (Variables|/Game/Individual_Work/Piper/WB_ViewMode.WB_ViewMode_C|GetViewtype (stale EventBeginPlay _returnvalue)) (Utilities|Text|ToText(String) _output)))))

(event Input|KeyboardEvents|7
  (params (Key :type Key%20Structure :default "None"))
  (bind _views (Variables|Default|GetViews))
  (bind _output (Utilities|Array|Get(acopy) _views 6))
  ;[0.15 0.15 0.15 0.5] Toggle through views
  (:Pressed
    (if (not (Variables|Default|GetPlayerPaused))
      (Development|ExecuteConsoleCommand _output 0)
      (Rendering|Components|TextRender|SetText (Variables|/Game/Individual_Work/Piper/WB_ViewMode.WB_ViewMode_C|GetViewtype (stale EventBeginPlay _returnvalue)) (Utilities|Text|ToText(String) _output)))))

(event Input|KeyboardEvents|8
  (params (Key :type Key%20Structure :default "None"))
  (bind _views (Variables|Default|GetViews))
  (bind _output (Utilities|Array|Get(acopy) _views 7))
  ;[0.15 0.15 0.15 0.5] Toggle through views
  (:Pressed
    (if (not (Variables|Default|GetPlayerPaused))
      (Development|ExecuteConsoleCommand _output 0)
      (Rendering|Components|TextRender|SetText (Variables|/Game/Individual_Work/Piper/WB_ViewMode.WB_ViewMode_C|GetViewtype (stale EventBeginPlay _returnvalue)) (Utilities|Text|ToText(String) _output)))))

(fn ConstructionScript)

(fn FootstepsTrace
  (bind _returnvalue (Transformation|GetActorLocation))
  (bind (_x _y _z) (Math|Vector|BreakVector _returnvalue))
  (bind (_outhit _returnvalue_2) (Collision|SphereTraceByChannel _returnvalue (Math|Vector|MakeVector _x _y (- _z (Components|Capsule|GetScaledCapsuleHalfHeight (Variables|Collision|GetCapsuleComponent)))) (Components|Capsule|GetScaledCapsuleRadius (Variables|Collision|GetCapsuleComponent)) "TraceTypeQuery1" false 0 "None"))
  (if _returnvalue_2
    (Variables|Default|SetHitResultLocation (.Location (Collision|BreakHitResult _outhit)))
    (if (Variables|Default|GetEscalator)
      (Audio|PlaySoundatLocation "/Game/Individual_Work/Piper/Sounds/Foley/SC_EscalatorFootsteps.SC_EscalatorFootsteps" (Variables|Default|GetHitResultLocation) "0, 0, 0" 1.0 1.0 0.0 0 0 0 0)
      (elif (Variables|Default|GetMetal)
        (Audio|PlaySoundatLocation "/Game/Individual_Work/Piper/Sounds/Sounds_Foley_AMB_SFX/Sounds_Foley_AMB_SFX/Foley/Metal_Footsteps/SC_FOL_Metal_Footsteps.SC_FOL_Metal_Footsteps" (Variables|Default|GetHitResultLocation) "0, 0, 0" 1.0 1.0 0.0 0 0 0 0)
        (elif (Variables|Default|GetGravel)
          (Audio|PlaySoundatLocation "/Game/Individual_Work/Piper/Sounds/Sounds_Foley_AMB_SFX/Sounds_Foley_AMB_SFX/Foley/Gravel_Footsteps/SC_FOL_Gravel_Footsteps.SC_FOL_Gravel_Footsteps" (Variables|Default|GetHitResultLocation) "0, 0, 0" 1.0 1.0 0.0 0 0 0 0)
          (else
            (Audio|PlaySoundatLocation "/Game/Individual_Work/Piper/Sounds/Foley/SC_TileFootsteps.SC_TileFootsteps" (Variables|Default|GetHitResultLocation) "0, 0, 0" 1.0 1.0 0.0 0 0 0 0)))))))