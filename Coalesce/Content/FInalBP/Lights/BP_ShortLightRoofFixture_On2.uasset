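; Roof fixture light actor with two short tube bulbs and a point light, able to switch its bulb glow off.
; On BeginPlay it creates dynamic material instances for both bulb meshes and gives the point light a slightly random cool color temperature.
; The TurnOffTubeLights event sets both materials' emission intensity to zero, leaving the point light itself untouched.
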(event Custom|TurnOffTubeLights
  ;[0.8879 0.4678 0.6445 0.502] Set light emmision intensity to 0
  (Utilities|FlowControl|Sequence
    (:then_0
      (Rendering|Material|SetScalarParameterValue (Variables|Default|GetDyn%20Mat%201) "Emission Intensity" 0.0 :!class /Script/Engine.MaterialInstanceDynamic))
    (:then_1
      (Rendering|Material|SetScalarParameterValue (Variables|Default|GetDyn%20Mat%202) "Emission Intensity" 0.0 :!class /Script/Engine.MaterialInstanceDynamic))))

(event EventBeginPlay
  ;[0.8879 0.4678 0.6445 0.502] Get Access to lights material
  (Utilities|FlowControl|Sequence
    (:then_0
      (bind _returnvalue (Rendering|Material|CreateDynamicMaterialInstance (Variables|Default|GetShortLightBlub_R) 0 0 "None" :!class /Script/Engine.PrimitiveComponent))
      (Variables|Default|SetDyn%20Mat%201 _returnvalue))
    (:then_1
      (bind _returnvalue_2 (Rendering|Material|CreateDynamicMaterialInstance (Variables|Default|GetShortLightBlub_L) 0 0 "None" :!class /Script/Engine.PrimitiveComponent))
      (Variables|Default|SetDyn%20Mat%202 _returnvalue_2))
    (:then_2
      ;[0.15 0.15 0.15 0.5] Random Lighting Temp
      (Class|LightComponent|SetTemperature (Variables|Default|GetPointLight) (Math|Random|RandomFloatinRange 6e+03 7e+03)))))

(fn ConstructionScript)