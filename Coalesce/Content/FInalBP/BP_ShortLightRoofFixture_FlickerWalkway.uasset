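; Roof light fixture Blueprint with two flickering bulb meshes and a point light that can be switched off.
; On BeginPlay it creates a dynamic material instance for the right and left bulb meshes.
; The TurnOffTubeLights event sets each material's FlickerTime parameter and the point light's intensity to zero.
; The graph has no logic to turn the lights back on.
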(event Custom|TurnOffTubeLights
  ;[0.8879 0.4678 0.6445 0.502] Set RectLight and Material emmision intensity to 0
  (Utilities|FlowControl|Sequence
    (:then_0
      (Rendering|Material|SetScalarParameterValue (Variables|Default|GetDynMat1) "FlickerTime" 0.0 :!class /Script/Engine.MaterialInstanceDynamic))
    (:then_1
      (Rendering|Material|SetScalarParameterValue (Variables|Default|GetDynMat2) "FlickerTime" 0.0 :!class /Script/Engine.MaterialInstanceDynamic))
    (:then_2
      (Rendering|Components|Light|SetIntensity (Variables|Default|GetPointLight) 0.0))))

(event EventBeginPlay
  ;[0.8879 0.4678 0.6445 0.502] Get access to lights material
  (Utilities|FlowControl|Sequence
    (:then_0
      (bind _returnvalue (Rendering|Material|CreateDynamicMaterialInstance (Variables|Default|GetShortLightBlub_R) 0 0 "None" :!class /Script/Engine.PrimitiveComponent))
      (Variables|Default|SetDynMat1 _returnvalue))
    (:then_1
      (bind _returnvalue_2 (Rendering|Material|CreateDynamicMaterialInstance (Variables|Default|GetShortLightBlub_L) 0 0 "None" :!class /Script/Engine.PrimitiveComponent))
      (Variables|Default|SetDynMat2 _returnvalue_2))))

(fn ConstructionScript)