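; BP_HFlickerLightWalkway is a walkway light that flickers continuously from BeginPlay.
; It creates dynamic emissive material instances for the left and right long bulb meshes, then loops on a short random Delay.
; Each pass randomizes the point light intensity and both bulbs' normalized emission separately, so glow and light output do not match.
; A random start-intensity branch is left unconnected and marked unused.
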(event EventBeginPlay
  (bind _returnvalue (Rendering|Material|CreateDynamicMaterialInstance (Variables|Default|GetLongLightBlub_L) 0 "/Game/Individual_Work/Shannon_B/Shaders/EmissiveLights/M_EmmisiveLights.M_EmmisiveLights" "None" :!class /Script/Engine.PrimitiveComponent))
  (bind _returnvalue_2 (Rendering|Material|CreateDynamicMaterialInstance (Variables|Default|GetLongLightBlub_R) 0 "/Game/Individual_Work/Shannon_B/Shaders/EmissiveLights/M_EmmisiveLights.M_EmmisiveLights" "None" :!class /Script/Engine.PrimitiveComponent))
  ;[0.15 0.15 0.15 0.5] The Light Intensity (Adjust)
  (bind _output_get (Variables|Default|SetNewIntensity 5e+02))
  ;[0.15 0.15 0.15 0.5] Normalizing the Emissive Material
  (bind _output_get_2 (Variables|Default|SetMinEmissive 0.0))
  (bind _output_get_3 (Variables|Default|SetMaxEmissive 1.0))
  (bind _output_get_4 (Variables|Default|SetDynMatBulbL _returnvalue :!label _label))
  (Rendering|Material|SetScalarParameterValue _output_get_4 "Emission Intensity" (Math|Float|Lerp _output_get_2 _output_get_3 (/ (Math|Random|RandomFloatinRange 0.0 _output_get) _output_get)) :!class /Script/Engine.MaterialInstanceDynamic)
  (bind _output_get_5 (Variables|Default|SetDynMatBulbR _returnvalue_2))
  (Rendering|Material|SetScalarParameterValue _output_get_5 "Emission Intensity" (Math|Float|Lerp _output_get_2 _output_get_3 (/ (Math|Random|RandomFloatinRange 0.0 _output_get) _output_get)) :!class /Script/Engine.MaterialInstanceDynamic)
  (Rendering|Components|Light|SetIntensity (Variables|Default|GetPointLight) (Math|Random|RandomFloatinRange 0.0 _output_get))
  (Utilities|FlowControl|Delay (Math|Random|RandomFloatinRange 0.05 0.5))
  (goto _label))

(fn ConstructionScript)