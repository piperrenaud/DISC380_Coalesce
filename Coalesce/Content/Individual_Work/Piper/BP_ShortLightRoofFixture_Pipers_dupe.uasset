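; BP_ShortLightRoofFixture_Pipers_dupe is a short roof light fixture whose two bulb meshes can be switched off visually.
; On BeginPlay it creates a dynamic material instance for the left and right bulbs and stores both.
; The TurnOffLight event sets the scalar emissive parameter "Param" to zero on both, so the glow is removed through the material alone.
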(event Custom|TurnOffLight
  ;[0.15 0.15 0.15 0.5] Turn off lights via emissive output
  (Utilities|FlowControl|Sequence
    (:then_0
      (Rendering|Material|SetScalarParameterValue (Variables|Default|GetDynMat_1) "Param" 0.0 :!class /Script/Engine.MaterialInstanceDynamic))
    (:then_1
      (Rendering|Material|SetScalarParameterValue (Variables|Default|GetDynMat_2) "Param" 0.0 :!class /Script/Engine.MaterialInstanceDynamic))))

(event EventBeginPlay
  ;[0.15 0.15 0.15 0.5] Get access to lights emission (Emissive color must be a scalar parameter)
  (Utilities|FlowControl|Sequence
    (:then_0
      (bind _returnvalue (Rendering|Material|CreateDynamicMaterialInstance (Variables|Default|GetShortLightBlub_L) 0 0 "None" :!class /Script/Engine.PrimitiveComponent))
      (Variables|Default|SetDynMat_1 _returnvalue))
    (:then_1
      (bind _returnvalue_2 (Rendering|Material|CreateDynamicMaterialInstance (Variables|Default|GetShortLightBlub_R) 0 0 "None" :!class /Script/Engine.PrimitiveComponent))
      (Variables|Default|SetDynMat_2 _returnvalue_2))))

(fn ConstructionScript)