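; Parent Blueprint for inspectable objects that the player can rotate with the mouse during inspection.
; StartInspect moves input from the inspecting actor to this object, and pressing Interact hands it back and calls Inspect on BP_Player.
; While either mouse button is held, mouse X and Y movement adjust the Item component's relative roll and pitch through combined rotators.
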(event Custom|StartInspect
  (params (Inspecter :type Pawn%20Object%20Reference))
  (bind _returnvalue (Game|GetPlayerController 0))
  ;[0.15 0.15 0.15 0.5] Start/Stop Inspect
  (Input|DisableInput Inspecter _returnvalue)
  (Input|EnableInput _returnvalue))

(event Input|ActionEvents|InputActionInteract
  (params (Key :type Key%20Structure :default "None"))
  (bind _returnvalue (Game|GetPlayerController 0))
  ;[0.15 0.15 0.15 0.5] Start/Stop Inspect
  (:Pressed
    (Input|DisableInput _returnvalue)
    (Input|EnableInput (stale Custom|StartInspect Inspecter) _returnvalue)
    (bind _asbp_player (Utilities|Casting|CastToBP_Player (stale Custom|StartInspect Inspecter)))
    (Default|Inspect _asbp_player)))

(event Input|MouseEvents|MouseX
  (params (AxisValue :type Float%20%28single-precision%29))
  (bind _returnvalue (Game|GetPlayerController 0))
  ;[0.15 0.15 0.15 0.5] Inspect Item w/ left or right mouse button
  (if (or (Game|Player|IsInputKeyDown _returnvalue "LeftMouseButton") (Game|Player|IsInputKeyDown _returnvalue "RightMouseButton"))
    (Transformation|SetRelativeRotation (Variables|Default|GetItem) (Math|Rotator|CombineRotators (Variables|/Script/Engine.SceneComponent|GetRelativeRotation (Variables|Default|GetItem)) (Math|Rotator|MakeRotator (* AxisValue -1.0) 0.0 0.0)) false false)))

(event Input|MouseEvents|MouseY
  (params (AxisValue :type Float%20%28single-precision%29))
  (bind _returnvalue (Game|GetPlayerController 0))
  ;[0.15 0.15 0.15 0.5] Inspect Item w/ left or right mouse button
  (if (or (Game|Player|IsInputKeyDown _returnvalue "LeftMouseButton") (Game|Player|IsInputKeyDown _returnvalue "RightMouseButton"))
    (Transformation|SetRelativeRotation (Variables|Default|GetItem) (Math|Rotator|CombineRotators (Variables|/Script/Engine.SceneComponent|GetRelativeRotation (Variables|Default|GetItem)) (Math|Rotator|MakeRotator 0.0 (* AxisValue -1.0) 0.0)) false false)))

(fn ConstructionScript)